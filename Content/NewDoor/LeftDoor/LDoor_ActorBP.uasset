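; Left door actor that opens by animation once the player has killed enough Gnawmers and holds enough keys.
; Tick casts the player pawn to ThirdPersonCharacter and polls its DeadGnawmers and Keys counts against fixed thresholds.
; When both are met, a DoOnce plays the non-looping door animation on LdoorRig.
; An unconnected copy of that DoOnce and animation call never runs.
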(event `self.ReceiveBeginPlay`)

(event `self.ReceiveActorBeginOverlap`
  (params (OtherActor :type "Actor Object Reference")))

(event `self.ReceiveTick`
  (params (DeltaSeconds :type "Float (single-precision)"))
  (bind _asthird_person_character (cast `/Game/ThirdPersonBP/Blueprints/ThirdPersonCharacter` (`GameplayStatics.GetPlayerCharacter` 0)))
  (if (>= (`/Game/ThirdPersonBP/Blueprints/ThirdPersonCharacter.DeadGnawmers` _asthird_person_character) 6.0)
    (if (>= (`/Game/ThirdPersonBP/Blueprints/ThirdPersonCharacter.Keys` _asthird_person_character) 4)
      (`/Engine/EditorBlueprintResources/StandardMacros.DoOnce` false
        (:`Completed`
          (`SkeletalMeshComponent.PlayAnimation` (`self.Ldoor_rig`) "/Game/NewDoor/LeftDoor/Ldoor_rig_Anim.Ldoor_rig_Anim" false))))))

(fn `UserConstructionScript`)