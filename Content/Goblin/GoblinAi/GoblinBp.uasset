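; GoblinBp is an AI goblin character that chases, attacks and dies with a ragdoll.
; The Sight1 volume toggles the IsChasing blackboard key, while PawnSensing moves it toward any other GoblinBp it sees.
; The Attacking volume plays a thrust animation and sets IsAttacking, never cleared here, which lets capsule overlaps damage ThirdPersonCharacter.
; Tick switches walk speed on IsRunning and, at zero Health, starts ragdoll physics before delayed destruction.
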(event `self.ReceiveBeginPlay`)

(event `self.ReceiveActorBeginOverlap`
  (params (OtherActor :type "Actor Object Reference")))

(event `self.Sight1.OnComponentBeginOverlap`
  (params (OtherActor :type "Actor Object Reference") (OtherComp :type "PrimitiveComponent Object Reference") (OtherBodyIndex :type Integer) (bFromSweep :type Boolean) (SweepResult :type "HitResult Structure (by ref)"))
  ;[1 1 1] Trigger Blackboard
  (`BlackboardComponent.SetValueAsBool` (`AIBlueprintHelperLibrary.GetBlackboard` self) "IsChasing" true))

(event `self.PawnSensing.OnSeePawn`
  (params (Pawn :type "Pawn Object Reference"))
  ;[1 1 1] GoblinAi moving around
  (bind _asgoblin_bp (cast `/Game/Goblin/GoblinAi/GoblinBp` Pawn))
  (`|AIMoveTo` self (0.0 0.0 0.0) _asgoblin_bp 10.0))

(event `self.Sight1.OnComponentEndOverlap`
  (params (OtherActor :type "Actor Object Reference") (OtherComp :type "PrimitiveComponent Object Reference") (OtherBodyIndex :type Integer))
  ;[1 1 1] Trigger Blackboard
  (`BlackboardComponent.SetValueAsBool` (`AIBlueprintHelperLibrary.GetBlackboard` self) "IsChasing" false))

(event `self.ReceiveTick`
  (params (DeltaSeconds :type "Float (single-precision)"))
  (bind _charactermovement (`self.CharacterMovement`))
  ;[1 1 1] if else character movement and rag doll effect
  (if (`self.IsRunning`)
    (set `CharacterMovementComponent.MaxWalkSpeed` 350.0 _charactermovement)
    (else
      (set `CharacterMovementComponent.MaxWalkSpeed` 150.0 _charactermovement)))
  (if (<= (`self.Health`) 0.0)
    (`PrimitiveComponent.SetCollisionEnabled` (`self.CapsuleComponent`) "NoCollision")
    (`PrimitiveComponent.SetSimulatePhysics` (`self.Mesh`) true)
    (`KismetSystemLibrary.Delay` 3.0)
    (`self.K2_DestroyActor`)))

(event `self.CapsuleComponent.OnComponentBeginOverlap`
  (params (OtherActor :type "Actor Object Reference") (OtherComp :type "PrimitiveComponent Object Reference") (OtherBodyIndex :type Integer) (bFromSweep :type Boolean) (SweepResult :type "HitResult Structure (by ref)"))
  ;[1 1 1] Damage Player
  (if (`self.IsAttacking`)
    (bind _asthird_person_character (cast `/Game/ThirdPersonBP/Blueprints/ThirdPersonCharacter` OtherActor))
    (set `/Game/ThirdPersonBP/Blueprints/ThirdPersonCharacter.PlayerHealth` (- (`/Game/ThirdPersonBP/Blueprints/ThirdPersonCharacter.PlayerHealth` _asthird_person_character) 0.03) _asthird_person_character)))

(event `self.Attacking.OnComponentBeginOverlap`
  (params (OtherActor :type "Actor Object Reference") (OtherComp :type "PrimitiveComponent Object Reference") (OtherBodyIndex :type Integer) (bFromSweep :type Boolean) (SweepResult :type "HitResult Structure (by ref)"))
  ;[1 1 1] Attack Player in box
  (cast `/Game/ThirdPersonBP/Blueprints/ThirdPersonCharacter` OtherActor)
  (set `self.IsAttacking` true)
  (`SkeletalMeshComponent.PlayAnimation` (`self.Mesh`) "/Game/Goblin/upward_thrust.upward_thrust" true)
  (`KismetSystemLibrary.Delay` 2.33)
  (`SkeletalMeshComponent.SetAnimationMode` (`self.Mesh`) "AnimationBlueprint"))

(fn `UserConstructionScript`)