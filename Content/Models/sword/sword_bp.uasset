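; Sword weapon Blueprint that damages actors its capsule begins overlapping, skipping any tagged Player.
; Each hit applies damage using its Damage and DamageType variables, then casts the player character to ThirdPersonCharacter and adds a fixed amount to the HUD's experience value.
; An Enemeies array guards against repeat hits, but is cleared right after each successful hit, so it does not persist between overlaps.
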(event `self.Capsule.OnComponentBeginOverlap`
  (params (OtherActor :type "Actor Object Reference") (OtherComp :type "PrimitiveComponent Object Reference") (OtherBodyIndex :type Integer) (bFromSweep :type Boolean) (SweepResult :type "EngineTypes.HitResult Structure (by ref)"))
  (if (`self.ActorHasTag` OtherActor "Player")
    _
    (elif (not (`KismetArrayLibrary.Array_Contains` (`self.Enemeies`) OtherActor))
      (`KismetArrayLibrary.Array_Add` (`self.Enemeies`) OtherActor)
      (`GameplayStatics.ApplyDamage` OtherActor (`self.Damage`) null self "/Script/Engine.DamageType")
      (bind _asthird_person_character (cast `/Game/ThirdPersonBP/Blueprints/ThirdPersonCharacter` (`GameplayStatics.GetPlayerCharacter` 0)))
      (bind _gamehud (`/Game/ThirdPersonBP/Blueprints/ThirdPersonCharacter.GameHud` _asthird_person_character))
      (set `/Game/GUI/Gui.H_Experience` (+ (`/Game/GUI/Gui.H_Experience` _gamehud) 0.1) _gamehud)
      (`KismetArrayLibrary.Array_Clear` (`self.Enemeies`)))))

(event `self.ReceiveBeginPlay`)

(event `self.ReceiveTick`
  (params (DeltaSeconds :type "Float (single-precision)")))

(fn `UserConstructionScript`)