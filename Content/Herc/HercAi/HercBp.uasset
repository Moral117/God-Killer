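; Herc enemy AI character that chases and hurts the player, with a shield and health linked to crystals.
; Overlap volumes set the IsChasing blackboard key, play the uppercut animation and subtract PlayerHealth on body contact.
; Tick swaps the shield material by Crystal2 life, derives Health from Crystal3, sets walk speed and handles animated death.
; Shield-contact damage casts one actor to both Crystal2 and player, so it cannot land as wired.
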(event `self.ReceiveBeginPlay`)

(event `self.ReceiveActorBeginOverlap`
  (params (OtherActor :type "Actor Object Reference")))

(event `self.Attack.OnComponentBeginOverlap`
  (params (OtherActor :type "Actor Object Reference") (OtherComp :type "PrimitiveComponent Object Reference") (OtherBodyIndex :type Integer) (bFromSweep :type Boolean) (SweepResult :type "HitResult Structure (by ref)"))
  ;[1 1 1] Play attack at overlay
  (cast `/Game/ThirdPersonBP/Blueprints/ThirdPersonCharacter` OtherActor)
  (`SkeletalMeshComponent.PlayAnimation` (`self.Mesh`) "/Game/Herc/back_flip_to_uppercut.back_flip_to_uppercut" true)
  (`KismetSystemLibrary.Delay` 3.16)
  (`SkeletalMeshComponent.SetAnimationMode` (`self.Mesh`) "AnimationBlueprint"))

(event `self.Sights.OnComponentBeginOverlap`
  (params (OtherActor :type "Actor Object Reference") (OtherComp :type "PrimitiveComponent Object Reference") (OtherBodyIndex :type Integer) (bFromSweep :type Boolean) (SweepResult :type "HitResult Structure (by ref)"))
  ;[1 1 1] Trigger Blackboard isChasing
  (`BlackboardComponent.SetValueAsBool` (`AIBlueprintHelperLibrary.GetBlackboard` self) "IsChasing" true))

(event `self.Sights.OnComponentEndOverlap`
  (params (OtherActor :type "Actor Object Reference") (OtherComp :type "PrimitiveComponent Object Reference") (OtherBodyIndex :type Integer))
  ;[1 1 1] Trigger Blackboard isChasing
  (`BlackboardComponent.SetValueAsBool` (`AIBlueprintHelperLibrary.GetBlackboard` self) "IsChasing" false))

(event `SheildColor`
  ;[1 1 1] Emmits particle for sheild
  (bind _ascrystal_2 (cast `/Game/Crysral11/Crystal2` (`self.Actor`)))
  (if (<= (`/Game/Crysral11/Crystal2.Life` _ascrystal_2) 0.0)
    (`/Engine/EditorBlueprintResources/StandardMacros.DoOnce` true
      (:`Completed`
        (`PrimitiveComponent.SetMaterial` (`self.Sheild`) 0 "/Game/Materials/HercSheildInvisible_Mat.HercSheildInvisible_Mat")))
    (else
      (`/Engine/EditorBlueprintResources/StandardMacros.DoOnce` false
        (:`Completed`
          (`PrimitiveComponent.SetMaterial` (`self.Sheild`) 0 "/Game/Materials/HercSheild_Mat.HercSheild_Mat"))))))

(event `self.ReceiveTick`
  (params (DeltaSeconds :type "Float (single-precision)"))
  (bind _charactermovement (`self.CharacterMovement`))
  ;[1 1 1] if else character movement and rag doll effect
  (`self.SheildColor`)
  (`self.Health Regeneration`)
  (if (`self.IsRunning`)
    (set `CharacterMovementComponent.MaxWalkSpeed` 350.0 _charactermovement)
    (else
      (set `CharacterMovementComponent.MaxWalkSpeed` 150.0 _charactermovement)))
  (if (<= (`self.Health`) 0.0)
    (`NavMovementComponent.StopActiveMovement` (`self.CharacterMovement`))
    (`SkeletalMeshComponent.PlayAnimation` (`self.Mesh`) "/Game/Herc/zombie_death.zombie_death" false)
    (`KismetSystemLibrary.Delay` 3.0)
    (`self.K2_DestroyActor`)))

(event `self.CapsuleComponent.OnComponentBeginOverlap`
  (params (OtherActor :type "Actor Object Reference") (OtherComp :type "PrimitiveComponent Object Reference") (OtherBodyIndex :type Integer) (bFromSweep :type Boolean) (SweepResult :type "HitResult Structure (by ref)"))
  ;[1 1 1] Damage Player
  (bind _asthird_person_character (cast `/Game/ThirdPersonBP/Blueprints/ThirdPersonCharacter` OtherActor))
  (set `/Game/ThirdPersonBP/Blueprints/ThirdPersonCharacter.PlayerHealth` (- (`/Game/ThirdPersonBP/Blueprints/ThirdPersonCharacter.PlayerHealth` _asthird_person_character) 0.05) _asthird_person_character))

(event `self.SheildCollision.OnComponentBeginOverlap`
  (params (OtherActor :type "Actor Object Reference") (OtherComp :type "PrimitiveComponent Object Reference") (OtherBodyIndex :type Integer) (bFromSweep :type Boolean) (SweepResult :type "HitResult Structure (by ref)"))
  ;[1 1 1] Force Feild
  (bind _ascrystal_2 (cast `/Game/Crysral11/Crystal2` OtherActor))
  (if (not (<= (`/Game/Crysral11/Crystal2.Life` _ascrystal_2) 0.0))
    (bind _asthird_person_character (cast `/Game/ThirdPersonBP/Blueprints/ThirdPersonCharacter` OtherActor))
    (bind _output_get (set `/Game/ThirdPersonBP/Blueprints/ThirdPersonCharacter.PlayerHealth` (- (`/Game/ThirdPersonBP/Blueprints/ThirdPersonCharacter.PlayerHealth` _asthird_person_character) 0.04) _asthird_person_character))
    (`KismetSystemLibrary.PrintString` (`KismetStringLibrary.Conv_DoubleToString` _output_get))))

(event `self.ReceiveAnyDamage`
  (params (Damage :type "Float (single-precision)") (DamageType :type "DamageType Object Reference") (InstigatedBy :type "Controller Object Reference") (DamageCauser :type "Actor Object Reference"))
  ;[1 1 1] HercHealth
)

(event `Health Regeneration`
  ;[1 1 1] Regenerates health(not connected to crystal yet)
  (bind _ascrystal_3 (cast `/Game/Crysral11/Crystal3` (`self.Crystal3`)))
  (if (<= (`/Game/Crysral11/Crystal3.Life` _ascrystal_3) 0.9)
    (set `self.Health` (+ (`/Game/Crysral11/Crystal3.Life` _ascrystal_3) 0.2))))

(fn `UserConstructionScript`)