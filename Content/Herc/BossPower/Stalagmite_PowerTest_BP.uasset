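; Boss power stalagmite test actor that damages the player on contact, judging by its name and path.
; Any overlap with its Box sets a 0.2 second lifespan, then checks whether player character 0 is inside.
; A DoOnce subtracts StalagmiteDamage from the ThirdPersonCharacter's PlayerHealth a single time.
; The follow-up delay that zeroes the damage outlasts that lifespan, and the component-destroy branch is disconnected.
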(event `self.ReceiveBeginPlay`)

(event `self.ReceiveActorBeginOverlap`
  (params (OtherActor :type "Actor Object Reference")))

(event `self.ReceiveTick`
  (params (DeltaSeconds :type "Float (single-precision)")))

(event `self.Box.OnComponentBeginOverlap`
  (params (OtherActor :type "Actor Object Reference") (OtherComp :type "PrimitiveComponent Object Reference") (OtherBodyIndex :type Integer) (bFromSweep :type Boolean) (SweepResult :type "HitResult Structure (by ref)"))
  ;[1 1 1] MakesStalagmiteDoDamage
  (`self.SetLifeSpan` 0.2)
  (if (`PrimitiveComponent.IsOverlappingActor` (`self.Box`) (`GameplayStatics.GetPlayerCharacter` 0))
    (`/Engine/EditorBlueprintResources/StandardMacros.DoOnce` false
      (:`Completed`
        (bind _asthird_person_character (cast `/Game/ThirdPersonBP/Blueprints/ThirdPersonCharacter` (`GameplayStatics.GetPlayerCharacter` 0)))
        (set `/Game/ThirdPersonBP/Blueprints/ThirdPersonCharacter.PlayerHealth` (- (`/Game/ThirdPersonBP/Blueprints/ThirdPersonCharacter.PlayerHealth` _asthird_person_character) (`self.Stalagmite_Damage`)) _asthird_person_character)
        (`KismetSystemLibrary.Delay` 0.25)
        (set `self.Stalagmite_Damage` 0.0)
        (`KismetSystemLibrary.Delay` 3.0)))))

(fn `UserConstructionScript`)