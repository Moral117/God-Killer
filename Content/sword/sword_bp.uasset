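; Sword weapon Blueprint that damages enemies it overlaps.
; Separate collision components each handle one enemy class: skeleton, three AlterSkel variants, goblin, kobold and Herc.
; Each overlap event casts the other actor to that class and subtracts a hard-coded amount directly from its Health or Life variable, without the engine damage system.
; BeginPlay, Tick and the construction script are empty.
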(event `self.ReceiveBeginPlay`)

(event `self.ReceiveTick`
  (params (DeltaSeconds :type "Float (single-precision)")))

(event `self.Capsule.OnComponentBeginOverlap`
  (params (OtherActor :type "Actor Object Reference") (OtherComp :type "PrimitiveComponent Object Reference") (OtherBodyIndex :type Integer) (bFromSweep :type Boolean) (SweepResult :type "HitResult Structure (by ref)"))
  ;[1 1 1] Damage Skeleton
  (bind _asskeleton_enemy_bp (cast `/Game/Key/Skeleton/NewModel/SkeletonAi/Skeleton_EnemyBP` OtherActor))
  (set `/Game/Key/Skeleton/NewModel/SkeletonAi/Skeleton_EnemyBP.Health` (- (`/Game/Key/Skeleton/NewModel/SkeletonAi/Skeleton_EnemyBP.Health` _asskeleton_enemy_bp) 1) _asskeleton_enemy_bp))

(event `self.DamageSkeleton1.OnComponentBeginOverlap`
  (params (OtherActor :type "Actor Object Reference") (OtherComp :type "PrimitiveComponent Object Reference") (OtherBodyIndex :type Integer) (bFromSweep :type Boolean) (SweepResult :type "HitResult Structure (by ref)"))
  ;[1 1 1] Damage AlterSkel1
  (bind _asalter_skel_1 (cast `/Game/SkeletonForAltar/AlterSkel1` OtherActor))
  (set `/Game/SkeletonForAltar/AlterSkel1.Life` (- (`/Game/SkeletonForAltar/AlterSkel1.Life` _asalter_skel_1) 3.0) _asalter_skel_1))

(event `self.DamageGoblin.OnComponentBeginOverlap`
  (params (OtherActor :type "Actor Object Reference") (OtherComp :type "PrimitiveComponent Object Reference") (OtherBodyIndex :type Integer) (bFromSweep :type Boolean) (SweepResult :type "HitResult Structure (by ref)"))
  ;[1 1 1] Damage to Goblin
  (bind _asgoblin_bp (cast `/Game/Goblin/GoblinAi/GoblinBp` OtherActor))
  (set `/Game/Goblin/GoblinAi/GoblinBp.Health` (- (`/Game/Goblin/GoblinAi/GoblinBp.Health` _asgoblin_bp) 1.0) _asgoblin_bp))

(event `self.DamageSkeleton2.OnComponentBeginOverlap`
  (params (OtherActor :type "Actor Object Reference") (OtherComp :type "PrimitiveComponent Object Reference") (OtherBodyIndex :type Integer) (bFromSweep :type Boolean) (SweepResult :type "HitResult Structure (by ref)"))
  ;[1 1 1] Damage AlterSkel2
  (bind _asalter_skel_2 (cast `/Game/SkeletonForAltar/AlterSkel2` OtherActor))
  (set `/Game/SkeletonForAltar/AlterSkel2.Life` (- (`/Game/SkeletonForAltar/AlterSkel2.Life` _asalter_skel_2) 0.03) _asalter_skel_2))

(event `self.DamageKobold.OnComponentBeginOverlap`
  (params (OtherActor :type "Actor Object Reference") (OtherComp :type "PrimitiveComponent Object Reference") (OtherBodyIndex :type Integer) (bFromSweep :type Boolean) (SweepResult :type "HitResult Structure (by ref)"))
  ;[1 1 1] Damage Kobold
  (bind _askobold_bp (cast `/Game/Kobold/KoboldAi/KoboldBp` OtherActor))
  (set `/Game/Kobold/KoboldAi/KoboldBp.Health` (- (`/Game/Kobold/KoboldAi/KoboldBp.Health` _askobold_bp) 1.0) _askobold_bp))

(event `self.DamageSkeleton3.OnComponentBeginOverlap`
  (params (OtherActor :type "Actor Object Reference") (OtherComp :type "PrimitiveComponent Object Reference") (OtherBodyIndex :type Integer) (bFromSweep :type Boolean) (SweepResult :type "HitResult Structure (by ref)"))
  ;[1 1 1] Damage AlterSkel3
  (bind _asalter_skel_3 (cast `/Game/SkeletonForAltar/AlterSkel3` OtherActor))
  (set `/Game/SkeletonForAltar/AlterSkel3.Life` (- (`/Game/SkeletonForAltar/AlterSkel3.Life` _asalter_skel_3) 3.0) _asalter_skel_3))

(event `self.DamageHerc.OnComponentBeginOverlap`
  (params (OtherActor :type "Actor Object Reference") (OtherComp :type "PrimitiveComponent Object Reference") (OtherBodyIndex :type Integer) (bFromSweep :type Boolean) (SweepResult :type "HitResult Structure (by ref)"))
  ;[1 1 1] Damage Herc
  (bind _asherc_bp (cast `/Game/Herc/HercAi/HercBp` OtherActor))
  (set `/Game/Herc/HercAi/HercBp.Health` (- (`/Game/Herc/HercAi/HercBp.Health` _asherc_bp) 0.2) _asherc_bp))

(fn `UserConstructionScript`)